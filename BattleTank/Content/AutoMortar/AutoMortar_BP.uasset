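; AutoMortar_BP is an automated mortar emplacement Blueprint with a dome turret, a barrel and a health bar widget.
; On BeginPlay it initializes its TankAiming component with the barrel and dome as barrel and turret.
; It then casts its widget to HealthBar and passes itself as MyTank, reusing the tank aiming and health display setup.
; No firing or targeting logic appears in this graph.
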(event `self.ReceiveBeginPlay`
  (`TankAimingComponent.Initialize` (`self.TankAiming`) (`self.MortarBarrel`) (`self.MortarDome`))
  (`self.InitializeHealthBarWidget`))

(fn `InitializeHealthBarWidget`
  (bind _ashealth_bar (cast `/Game/UI/HealthBar` (`WidgetComponent.GetUserWidgetObject` (`self.Widget`))))
  (set `/Game/UI/HealthBar.MyTank` self _ashealth_bar))

(fn `UserConstructionScript`)